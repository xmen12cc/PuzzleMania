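; BP_Timer is a countdown timer actor in the RedLightGreenLight folder that shows its value through a W_Timer widget.
; BeginPlay casts the widget component's widget to W_Timer and caches it.
; Tick runs through a one-second Delay, so Timer drops by one about every second and is written to TimeText.
; The countdown has no lower limit or end event.
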(event `self.ReceiveTick`
  (params (DeltaSeconds :type "Float (single-precision)"))
  ;[1 1 1] Event tick and begin play with timer
  (`KismetSystemLibrary.Delay` 1.0)
  (bind _result (`/Engine/EditorBlueprintResources/StandardMacros.DecrementFloat` (`self.Timer`))
    (:`  `
      (bind _output_get (set `self.Timer` _result))
      (set `TextBlock.Text` (`KismetTextLibrary.Conv_StringToText` (`KismetStringLibrary.BuildString_Double` "" "" _output_get)) (`/Game/Blueprints/RedLightGreenLight/W_Timer.TimeText` (stale `self.ReceiveBeginPlay` _asw_timer))))))

(event `self.ReceiveBeginPlay`
  ;[1 1 1] Event tick and begin play with timer
  (bind _asw_timer (cast `/Game/Blueprints/RedLightGreenLight/W_Timer` (`WidgetComponent.GetWidget` (`self.Widget`)))))

(fn `UserConstructionScript`)