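; Game mode for Tic-Tac-Toe that assigns player IDs and the opening turn.
; After a short delay on BeginPlay, it gathers every BP_TicTacToePlayerController and numbers the first two by array index.
; The first controller found starts with the turn and the second waits, with each assignment printed for debugging.
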(event `self.ReceiveBeginPlay`
  (`KismetSystemLibrary.Delay` 2.0)
  (`self.AssignPlayerIDs`))

(event `AssignPlayerIDs`
  (bind _outactors (`GameplayStatics.GetAllActorsOfClass` "/Game/Blueprints/TicTacToe/BP_TicTacToePlayerController.BP_TicTacToePlayerController_C"))
  (for (_array_element _array_index) _outactors
    (switch `int` _array_index
      (:`0`
        (set `/Game/Blueprints/TicTacToe/BP_TicTacToePlayerController.PlayerID` 0 _array_element)
        (`KismetSystemLibrary.PrintString` "Assigned 0")
        (set `/Game/Blueprints/TicTacToe/BP_TicTacToePlayerController.IsMyTurn` true _array_element))
      (:`1`
        (set `/Game/Blueprints/TicTacToe/BP_TicTacToePlayerController.PlayerID` 1 _array_element)
        (`KismetSystemLibrary.PrintString` "Assigned 1")
        (set `/Game/Blueprints/TicTacToe/BP_TicTacToePlayerController.IsMyTurn` false _array_element)))))

(fn `UserConstructionScript`)