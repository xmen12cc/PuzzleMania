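; Game state for networked two-player tic-tac-toe, holding the grid, active player and game result.
; MakeMove rejects taken cells or inactive games, writes GridState, multicasts the board, then checks for a win.
; CheckWinCondition loops WinningCombos through hard-coded line comparisons, ending on a win or passing IsMyTurn to the next PlayerController; its partial draw check only sets IsDraw.
; Multicast events find the board widget by class to show marks and results.
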(event `Multicast_EndGame`
  ;[1 1 1] EndGame
  (bind _foundwidgets (`WidgetBlueprintLibrary.GetAllWidgetsOfClass` "/Game/Blueprints/TicTacToe/WBP_TicTacToeBoard.WBP_TicTacToeBoard_C"))
  (if (`self.isDraw`)
    (bind _winnertext (`/Game/Blueprints/TicTacToe/WBP_TicTacToeBoard.WinnerText` (`|GetArrayItem` _foundwidgets)))
    (set `TextBlock.Text` "Its a draw." _winnertext)
    (else
      (set `TextBlock.Text` (`KismetTextLibrary.Conv_StringToText` (`KismetStringLibrary.BuildString_Int` "" "Player" (+ (`self.CurrentPlayer`) 1) " Won!")) _winnertext))))

(event `Multicast_UpdateBoard`
  (params (Gridstate :type "Array of Integer"))
  ;[1 1 1] UpdateBoard
  (for (_array_element _array_index) Gridstate
    (switch `int` _array_element
      (:`-1`
        (bind _foundwidgets (`WidgetBlueprintLibrary.GetAllWidgetsOfClass` "/Game/Blueprints/TicTacToe/WBP_TicTacToeBoard.WBP_TicTacToeBoard_C"))
        (`/Game/Blueprints/TicTacToe/WBP_TicTacToeBoard.UpdateCellText` _foundwidgets _array_index ""))
      (:`0`
        (bind _foundwidgets_2 (`WidgetBlueprintLibrary.GetAllWidgetsOfClass` "/Game/Blueprints/TicTacToe/WBP_TicTacToeBoard.WBP_TicTacToeBoard_C"))
        (`/Game/Blueprints/TicTacToe/WBP_TicTacToeBoard.UpdateCellText` _foundwidgets_2 _array_index "X"))
      (:`1`
        (bind _foundwidgets_3 (`WidgetBlueprintLibrary.GetAllWidgetsOfClass` "/Game/Blueprints/TicTacToe/WBP_TicTacToeBoard.WBP_TicTacToeBoard_C"))
        (`/Game/Blueprints/TicTacToe/WBP_TicTacToeBoard.UpdateCellText` _foundwidgets_3 _array_index "O")))))

(event `MakeMove`
  (params (CellIndex :type Integer) (CurrentPlayer :type Integer))
  ;[1 1 1] MakeMove
  (if (`self.isGameActive`)
    (if (!= (`|GetArrayItem` (`self.GridState`) CellIndex) -1)
      (`KismetSystemLibrary.PrintString` "Row taken")
      (else
        (`KismetArrayLibrary.Array_Set` (`self.GridState`) CellIndex CurrentPlayer)
        (`self.Multicast_UpdateBoard` (`self.GridState`))
        (`self.CheckWinCondition`)))
    (else
      (`KismetSystemLibrary.PrintString` "Game is not active"))))

(event `CheckWinCondition`
  (bind _gridstate (`self.GridState`))
  (bind _gridstate_2 (`self.GridState`))
  (bind _gridstate_3 (`self.GridState`))
  (bind _gridstate_4 (`self.GridState`))
  (bind _gridstate_5 (`self.GridState`))
  (bind _gridstate_6 (`self.GridState`))
  (bind _gridstate_7 (`self.GridState`))
  (bind _gridstate_8 (`self.GridState`))
  (bind _output (`|GetArrayItem` _gridstate_8 6))
  (bind _output_2 (`|GetArrayItem` _gridstate 1))
  (bind _output_3 (`|GetArrayItem` _gridstate 2))
  (bind _output_4 (`|GetArrayItem` _gridstate_2 4))
  (bind _output_5 (`|GetArrayItem` _gridstate_2 5))
  (bind _output_6 (`|GetArrayItem` _gridstate_3 7))
  (bind _output_7 (`|GetArrayItem` _gridstate_3 8))
  (bind _output_8 (`|GetArrayItem` _gridstate_4 3))
  (bind _output_9 (`|GetArrayItem` _gridstate_4 6))
  (bind _output_10 (`|GetArrayItem` _gridstate_5 4))
  (bind _output_11 (`|GetArrayItem` _gridstate_5 7))
  (bind _output_12 (`|GetArrayItem` _gridstate_6 5))
  (bind _output_13 (`|GetArrayItem` _gridstate_6 8))
  (bind _output_14 (`|GetArrayItem` _gridstate_7 4))
  (bind _output_15 (`|GetArrayItem` _gridstate_8 4))
  (bind _output_16 (`|GetArrayItem` _gridstate_7 8))
  (bind _returnvalue (!= _output -1))
  (bind _returnvalue_2 (!= _output_3 -1))
  (bind _returnvalue_3 (!= _output_7 -1))
  (bind _returnvalue_4 (!= _output_9 -1))
  (bind _returnvalue_5 (!= _output_11 -1))
  (bind _returnvalue_6 (!= _output_13 -1))
  (bind _returnvalue_7 (!= _output_16 -1))
  (bind _returnvalue_8 (!= _output_5 -1))
  ;[1 1 1] CheckWinCondition
  (if (`self.isGameActive`)
    (for (_ _array_index) (`self.WinningCombos`)
      (if (== _array_index 0)
        (if (and (and (== (`|GetArrayItem` _gridstate) _output_2) (== _output_2 _output_3)) _returnvalue_2)
          (set `self.isGameActive` false :!label _label)
          (`self.Multicast_EndGame`))
        (elif (== _array_index 3)
          (if (and (and (== (`|GetArrayItem` _gridstate_2 3) _output_4) (== _output_4 _output_5)) _returnvalue_8)
            (goto _label))
          (elif (== _array_index 6)
            (if (and (and (== (`|GetArrayItem` _gridstate_3 6) _output_6) (== _output_6 _output_7)) _returnvalue_3)
              (goto _label))
            (elif (== _array_index 9)
              (if (and (and (== (`|GetArrayItem` _gridstate_4) _output_8) (== _output_8 _output_9)) _returnvalue_4)
                (goto _label))
              (elif (== _array_index 12)
                (if (and (and (== (`|GetArrayItem` _gridstate_5 1) _output_10) (== _output_10 _output_11)) _returnvalue_5)
                  (goto _label))
                (elif (== _array_index 14)
                  (if (and (and (== (`|GetArrayItem` _gridstate_6 2) _output_12) (== _output_12 _output_13)) _returnvalue_6)
                    (goto _label))
                  (elif (== _array_index 17)
                    (if (and (and (== (`|GetArrayItem` _gridstate_7) _output_14) (== _output_14 _output_16)) _returnvalue_7)
                      (goto _label))
                    (elif (== _array_index 20)
                      (if (and (and (== (`|GetArrayItem` _gridstate_8 2) _output_15) (== _output_15 _output)) _returnvalue)
                        (goto _label)
                        (elif (and (and (and _returnvalue_2 _returnvalue_8) (and _returnvalue_3 _returnvalue_4)) (and (and _returnvalue_5 _returnvalue_6) (and _returnvalue_7 _returnvalue)))
                          (set `self.isDraw` true))))))))))))
    (if (`self.isGameActive`)
      (if (== (`self.CurrentPlayer`) 0)
        (bind _output_get (set `self.CurrentPlayer` 1))
        (bind _asbp_tic_tac_toe_player_controller (cast `/Game/Blueprints/TicTacToe/BP_TicTacToePlayerController` (`GameplayStatics.GetPlayerController` _output_get)))
        (set `/Game/Blueprints/TicTacToe/BP_TicTacToePlayerController.IsMyTurn` true _asbp_tic_tac_toe_player_controller)
        (else
          (bind _output_get_2 (set `self.CurrentPlayer` 0))
          (bind _asbp_tic_tac_toe_player_controller_2 (cast `/Game/Blueprints/TicTacToe/BP_TicTacToePlayerController` (`GameplayStatics.GetPlayerController` _output_get_2)))
          (set `/Game/Blueprints/TicTacToe/BP_TicTacToePlayerController.IsMyTurn` true _asbp_tic_tac_toe_player_controller_2))))))

(fn `UserConstructionScript`)