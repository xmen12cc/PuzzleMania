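; BP_Tile is a floor tile for the Falling Floors game that drops away after a BP_FallingFloorsCharacter touches it.
; Box overlap by such a character, while the tile is not yet falling, triggers a color change and starts a delayed Multicast_TileFall.
; That event disables mesh collision, enables physics, plays a drop sound, then destroys the actor after a short delay.
; Server_TileFall and TileFall are similar immediate-destroy variants that nothing here calls.
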(event `self.ReceiveBeginPlay`
  (set `self.IsFalling` false))

(event `self.Box.OnComponentBeginOverlap`
  (params (OverlappedComponent :type "PrimitiveComponent Object Reference") (OtherActor :type "Actor Object Reference") (OtherComp :type "PrimitiveComponent Object Reference") (OtherBodyIndex :type Integer) (bFromSweep :type Boolean) (SweepResult :type "HitResult Structure (by ref)"))
  (bind _outactors (`GameplayStatics.GetAllActorsOfClass` "/Game/Blueprints/FallingFloors/BP_FallingFloorsCharacter.BP_FallingFloorsCharacter_C"))
  (for _array_element _outactors
    (if (== OtherActor _array_element)
      (if (== (`self.IsFalling`) false)
        (`self.Multicast_ChangeColor`)
        (`KismetSystemLibrary.K2_SetTimer` null "Multicast_TileFall" (`self.FallDelay`))
        (else
          (`KismetSystemLibrary.PrintString` "Not falling"))))))

(event `Server_TileFall`
  (set `self.IsFalling` true)
  (`PrimitiveComponent.SetCollisionEnabled` (`self.Box`) "NoCollision")
  (`PrimitiveComponent.SetCollisionEnabled` (`self.StaticMesh`) "NoCollision")
  (`PrimitiveComponent.SetSimulatePhysics` (`self.Box`) true)
  (`PrimitiveComponent.SetSimulatePhysics` (`self.StaticMesh`) true)
  (`self.K2_DestroyActor`))

(event `Multicast_TileFall`
  (set `self.IsFalling` true)
  (`PrimitiveComponent.SetCollisionEnabled` (`self.StaticMesh`) "NoCollision")
  (`PrimitiveComponent.SetSimulatePhysics` (`self.StaticMesh`) true)
  (`GameplayStatics.SpawnSoundAttached` "/Game/Sounds/FallingFloors/Drop.Drop" (`self.StaticMesh`) "None" (0.0 0.0 0.0) (struct) "KeepRelativeOffset" false 1.0 1.0 0.0 null null)
  (`KismetSystemLibrary.Delay` 1.2)
  (`self.K2_DestroyActor`))

(event `Multicast_ChangeColor`
  (`PrimitiveComponent.SetMaterial` (`self.StaticMesh`) 0 "/Game/Blueprints/FallingFloors/M_FloorTileDestroyed.M_FloorTileDestroyed"))

(event `TileFall`
  (set `self.IsFalling` true)
  (`PrimitiveComponent.SetCollisionEnabled` (`self.StaticMesh`) "NoCollision")
  (`PrimitiveComponent.SetCollisionEnabled` (`self.Box`) "NoCollision")
  (`PrimitiveComponent.SetSimulatePhysics` (`self.StaticMesh`) true)
  (`PrimitiveComponent.SetSimulatePhysics` (`self.Box`) true)
  (`self.K2_DestroyActor`))

(fn `UserConstructionScript`)