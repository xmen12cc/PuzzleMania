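; Game mode for the Falling Floors multiplayer minigame, handling arena setup and match start.
; On BeginPlay it spawns stacked grids of BP_Tile floors, then after a delay assigns player indices and places a BP_VoidBox below.
; When the ready count reaches two on login, a delayed multicast enables input and restores character gravity.
; Death updates log the player and decrement that same counter.
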(event `self.ReceiveBeginPlay`
  (`self.SpawnTiles`)
  (`KismetSystemLibrary.Delay` 3.0)
  (bind _outactors (`GameplayStatics.GetAllActorsOfClass` "/Game/Blueprints/FallingFloors/BP_FallingFloorsCharacter.BP_FallingFloorsCharacter_C"))
  (for (_array_element _array_index) _outactors
    (switch `int` _array_index
      (:`0`
        (set `/Game/Blueprints/FallingFloors/BP_FallingFloorsCharacter.PlayerIndex` 1 _array_element))
      (:`1`
        (set `/Game/Blueprints/FallingFloors/BP_FallingFloorsCharacter.PlayerIndex` 2 _array_element))
      (:`2`
        (set `/Game/Blueprints/FallingFloors/BP_FallingFloorsCharacter.PlayerIndex` 3 _array_element))
      (:`3`
        (set `/Game/Blueprints/FallingFloors/BP_FallingFloorsCharacter.PlayerIndex` 4 _array_element)))
    (`KismetSystemLibrary.PrintString` (`KismetStringLibrary.BuildString_Int` "" "Assigned " _array_index))
    (set `/Game/Blueprints/FallingFloors/BP_FallingFloorsCharacter.isAlive` true _array_element)
    (`|SpawnActorFromClass` "/Game/Blueprints/FallingFloors/BP_VoidBox.BP_VoidBox_C" (`KismetMathLibrary.MakeTransform` (0.0 0.0 -3600.0)) "Undefined" "MultiplyWithRoot" null null)))

(event `self.ReceiveTick`
  (params (DeltaSeconds :type "Float (single-precision)")))

(event `SpawnTiles`
  (bind _tilesize (`self.TileSize`))
  (bind _tilegap (`self.TileGap`))
  (for _index (range 1 (`self.LevelsCount`))
    (for _index_2 (range (`self.GridSizeX`))
      (for _index_3 (range (`self.GridSizeY`))
        (`|SpawnActorFromClass` "/Game/Blueprints/FallingFloors/BP_Tile.BP_Tile_C" (`KismetMathLibrary.MakeTransform` (`KismetMathLibrary.MakeVector` (* _index_3 (+ _tilesize _tilegap)) (* _index_2 (+ _tilesize _tilegap)) (* _index (`self.FloorHeight`))) (`KismetMathLibrary.MakeRotator` 0.0)) "Undefined" "MultiplyWithRoot" null null)))))

(event `PlayerReady()`
  (`/Engine/EditorBlueprintResources/StandardMacros.IncrementInt` (`self.PlayersReadyCount`)))

(event `self.K2_PostLogin`
  (params (NewPlayer :type "PlayerController Object Reference"))
  (bind _playersreadycount (`self.PlayersReadyCount`))
  (`/Engine/EditorBlueprintResources/StandardMacros.IncrementInt` _playersreadycount
    (:`  `
      (if (== _playersreadycount 2)
        (`KismetSystemLibrary.PrintString` (`KismetStringLibrary.Conv_IntToString` _playersreadycount))
        (`KismetSystemLibrary.Delay` 8.0)
        (`self.StartGame`)))))

(event `UpdatePlayerAlive`
  (params (Index :type Integer) (`Alive?` :type Boolean) (NewParam :type "/Game/Blueprints/FallingFloors/BP_FallingFloorsCharacter Object Reference"))
  (`KismetSystemLibrary.PrintString` (`KismetStringLibrary.BuildString_Int` "" "Player #" Index " Has died!"))
  (`/Engine/EditorBlueprintResources/StandardMacros.DecrementInt` (`self.PlayersReadyCount`)))

(event `StartGame`
  (`self.Multicast_StartGame`))

(event `Multicast_StartGame`
  (`self.EnableInput` null)
  (bind _outactors (`GameplayStatics.GetAllActorsOfClass` "/Game/Blueprints/FallingFloors/BP_FallingFloorsCharacter.BP_FallingFloorsCharacter_C"))
  (for _array_element _outactors
    (set `CharacterMovementComponent.GravityScale` 1.0 (`Character.CharacterMovement` _array_element))))

(fn `UserConstructionScript`)